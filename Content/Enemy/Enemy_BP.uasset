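; Enemy character that roams random reachable points, chases the player when seen by PawnSensing, and punches on arrival.
; Tick clears the chase shortly after sight lapses, which a retriggerable delay tracks, and AIMoveTo drives both movement modes.
; Punches lock movement and run a delayed, self-repeating capsule trace at the hand socket to damage the player.
; Hit reduces health, playing a damage montage or a death sound and montage before destroying the actor.
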(event OnSeePawn(PawnSensing)
  (params (Pawn :type Pawn%20Object%20Reference))
  ;[1 1 1] Chase player if sensed
  (bind _asthird_person_character (Utilities|Casting|CastToThirdPersonCharacter Pawn))
  (Utilities|FlowControl|Sequence
    (:then_0
      (Variables|Default|SetSeesEnemy true)
      (Variables|Default|SetIsChasing true)
      (Variables|/Script/Engine.CharacterMovementComponent|SetMaxWalkSpeed (Variables|Character|GetCharacterMovement) (Variables|Default|GetChaseSpeed))
      (AI|AIMoveTo self "0, 0, 0" _asthird_person_character 1e+01 false
        (:OnSuccess
          (CallFunction|Attack))))
    (:then_1
      (Utilities|FlowControl|RetriggerableDelay 0.6)
      (Variables|Default|SetSeesEnemy false))))

(event Custom|Hit
  ;[1 1 1] Take damage
  (Utilities|FlowControl|DoOnce false :!label _label
    (:Completed
      (Pawn|Components|CharacterMovement|DisableMovement (Variables|Character|GetCharacterMovement))
      (bind _output_get (Variables|Default|SetHealth (- (Variables|Default|GetHealth) (Variables|Default|GetDamage))))
      (if (> _output_get 0)
        (bind _returnvalue (Animation|PlayAnimMontage "/Game/Enemy/Anims/Enemy_Damage_1.Enemy_Damage_1" 1.5 "None"))
        (Pawn|Components|CharacterMovement|SetMovementMode (Variables|Character|GetCharacterMovement) "MOVE_Walking" 0)
        (goto _label Reset)
        (else
          (Audio|PlaySoundatLocation "/Game/Audio/Enemy_Death_SFX_Cue.Enemy_Death_SFX_Cue" (Transformation|GetActorLocation) "0, 0, 0" 1.0 1.0 0.0 0 0 0)
          (Variables|Default|SetIsDead true)
          (bind _returnvalue_2 (Animation|PlayAnimMontage "/Game/Enemy/Anims/Enemy_Death_1.Enemy_Death_1" 1.0 "None"))
          (Utilities|FlowControl|Delay _returnvalue_2)
          (Actor|DestroyActor))))))

(event Custom|Attack
  ;[1 1 1] Punching
  (if (and (not (Variables|Default|GetIsPunching)) (not (Variables|Default|GetIsDead)))
    (Variables|Default|SetIsPunching true)
    (Variables|Default|SetIsLeftHand false)
    (Pawn|Components|CharacterMovement|DisableMovement (Variables|Character|GetCharacterMovement))
    (bind _returnvalue (Animation|PlayAnimMontage "/Game/Enemy/Anims/Enemy_Punch_Anim_Montage.Enemy_Punch_Anim_Montage" 1.2 "None"))
    (Utilities|FlowControl|Sequence
      (:then_0
        (Utilities|FlowControl|Delay (/ _returnvalue 1.2))
        (Variables|Default|SetIsPunching false)
        (Pawn|Components|CharacterMovement|SetMovementMode (Variables|Character|GetCharacterMovement) "MOVE_Walking" 0))
      (:then_1
        (Utilities|FlowControl|Delay (/ _returnvalue 3.7))
        (CallFunction|AttackTrace)))))

(event Custom|AttackTrace
  (bind _mesh (Variables|Character|GetMesh))
  (bind _islefthand (Variables|Default|GetIsLeftHand))
  (bind _returnvalue (select _islefthand "LeftHand" "RightHand"))
  (bind _returnvalue_2 (Transformation|GetSocketLocation _mesh _returnvalue))
  ;[1 1 1] Punch Detection
  (if (Variables|Default|GetIsPunching)
    (bind (_outhit _returnvalue_3) (Class|KismetSystemLibrary|CapsuleTraceSingleforObjects _returnvalue_2 _returnvalue_2 22.0 22.0 (Utilities|Array|MakeArray "ObjectTypeQuery3") false 0 "None" true))
    (if _returnvalue_3
      (bind _asthird_person_character (Utilities|Casting|CastToThirdPersonCharacter (.HitActor (Collision|BreakHitResult _outhit))))
      (Default|TakeDamage _asthird_person_character)
      (else
        (Utilities|FlowControl|Delay 0.01)
        (CallFunction|AttackTrace)))))

(event EventBeginPlay
  ;[1 1 1] Default stuff
  (bind _asthird_person_character (Utilities|Casting|CastToThirdPersonCharacter (Game|GetPlayerCharacter 0)))
  (Variables|Default|SetCharacterReference _asthird_person_character))

(event EventTick
  (params (DeltaSeconds :type Float%20%28single-precision%29))
  ;[1 1 1] Roam
  (Utilities|FlowControl|Sequence
    (:then_0
      (if (not (Variables|Default|GetSeesEnemy))
        (Utilities|FlowControl|Delay 0.4)
        (if (not (Variables|Default|GetSeesEnemy))
          (Variables|Default|SetIsChasing false))))
    (:then_1
      (if (not (Variables|Default|GetIsChasing))
        (Utilities|FlowControl|Delay (Math|Random|RandomFloatinRange 2.0 5.0))
        (Variables|/Script/Engine.CharacterMovementComponent|SetMaxWalkSpeed (Variables|Character|GetCharacterMovement) (Variables|Default|GetRoamSpeed))
        (AI|AIMoveTo self (.RandomLocation (AI|Navigation|GetRandomReachablePointinRadius (Transformation|GetActorLocation) 1.5e+03 0 0)) 0 5.0 false)))))

(event Input|AxisEvents|InputAxisMoveForward
  (params (AxisValue :type Float%20%28single-precision%29))
  ;[1 1 1] Default stuff
  (Pawn|Input|AddMovementInput (Math|Vector|GetForwardVector (Math|Rotator|MakeRotator 0.0 0.0 (.Yaw (Math|Rotator|BreakRotator (Pawn|GetControlRotation :!class /Script/Engine.Pawn))))) AxisValue false))

(event Input|AxisEvents|InputAxisMoveRight
  (params (AxisValue :type Float%20%28single-precision%29))
  ;[1 1 1] Default stuff
  (Pawn|Input|AddMovementInput (Math|Vector|GetRightVector (Math|Rotator|MakeRotator 0.0 0.0 (.Yaw (Math|Rotator|BreakRotator (Pawn|GetControlRotation :!class /Script/Engine.Pawn))))) AxisValue false))

(fn ConstructionScript)